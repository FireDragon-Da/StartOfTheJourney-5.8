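; Linear dialogue trigger actor that opens a dialogue widget when its Box component is overlapped.
; The overlap creates WBP_DialogueLinear with the actor's DialogueTable, binds its finished event and adds it to the viewport; finishing removes it.
; Q advances the dialogue only while IsVisible is true, but both overlap and finish set it false, so nothing here enables advancing or blocks repeat widgets.
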(event OnComponentBeginOverlap(Box)
  (params (OverlappedComponent :type Primitive%20Component%20Object%20Reference) (OtherActor :type Actor%20Object%20Reference) (OtherComp :type Primitive%20Component%20Object%20Reference) (OtherBodyIndex :type Integer) (bFromSweep :type Boolean) (SweepResult :type Hit%20Result%20Structure%20%28by%20ref%29))
  (if (not (Variables|Default|GetisVisible))
    (bind _returnvalue (UserInterface|CreateWidget "/Game/Week8/WBP_DialogueLinear.WBP_DialogueLinear_C" (Game|GetPlayerController 0) (Variables|Default|GetDialogueTable)))
    (Variables|Default|SetDialogueWidget _returnvalue)
    (EventDispatchers|BindEventtoDialogueFinished (Variables|Default|GetDialogueWidget) (EventDispatchers|CreateEvent :!event Custom|HandleDialogueFinished))
    (UserInterface|Viewport|AddtoViewport (Variables|Default|GetDialogueWidget) 0)
    (Variables|Default|SetisVisible false)
    (if true
      _)))

(event Custom|HandleDialogueFinished
  (Widget|RemovefromParent (Variables|Default|GetDialogueWidget))
  (Variables|Default|SetisVisible false))

(event EventBeginPlay)

(event Collision|EventActorBeginOverlap
  (params (OtherActor :type Actor%20Object%20Reference)))

(event EventTick
  (params (DeltaSeconds :type Float%20%28single-precision%29)))

(event Input|KeyboardEvents|Q
  (params (Key :type Key%20Structure))
  (:Pressed
    (if (Variables|Default|GetisVisible)
      (Default|Advance (Variables|Default|GetDialogueWidget)))))

(fn ConstructionScript)

(fn BPDidlogueLinearAutoGenFunc)