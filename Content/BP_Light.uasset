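; BP_Light is a switchable spotlight, labeled by a text render that shows its LightIndex.
; The ToggleLights event flips IsOn and sets the spotlight's visibility to match.
; The construction script applies the same visibility from IsOn and writes the index into the text.
; A branch that would switch the cube's collision with IsOn is left disconnected and never runs.
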(event EventToggleLights
  (bind _output_get (Variables|Default|SetisOn? (not (Variables|Default|GetisOn?))))
  (Rendering|SetVisibility (Variables|Default|GetSpotLight) _output_get false))

(fn ConstructionScript
  (Rendering|SetVisibility (Variables|Default|GetSpotLight) (Variables|Default|GetisOn?) false)
  (Rendering|Components|TextRender|SetText (Variables|Default|GetTextRender) (Utilities|Text|ToText(Integer) (Variables|Default|GetlightIndex))))