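; BP_LightSwitch is a proximity-based switch that toggles the lights sharing its LightIndex.
; On BeginPlay it caches every BP_Light in the level into LightArray.
; Overlap begin and end enable or disable player input and open or close a Gate.
; Pressing C while the Gate is open calls ToggleLightsMessage on each cached light with a matching index.
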(event EventBeginPlay
  (bind _outactors (Actor|GetAllActorsOfClass "/Game/BP_Light.BP_Light_C"))
  (for _array_element _outactors
    (Utilities|Array|Add (Variables|Default|GetlightArray) _array_element)))

(event Collision|EventActorBeginOverlap
  (params (OtherActor :type Actor%20Object%20Reference))
  (Input|EnableInput (Game|GetPlayerController 0))
  (Utilities|FlowControl|Gate true) ; enters at Open
)

(event Collision|EventActorEndOverlap
  (params (OtherActor :type Actor%20Object%20Reference))
  (Input|DisableInput (Game|GetPlayerController 0))
  (Utilities|FlowControl|Gate true) ; enters at Close
)

(event Input|KeyboardEvents|C
  (params (Key :type Key%20Structure :default "None"))
  (:Pressed
    (Utilities|FlowControl|Gate true
      (:Exit
        (for _array_element (Variables|Default|GetlightArray)
          (if (== (Variables|/Game/BP_Light.BP_Light_C|GetlightIndex _array_element) (Variables|Default|GetlightIndex))
            (Class|BPILight|ToggleLights(Message) _array_element)))))))

(fn ConstructionScript)