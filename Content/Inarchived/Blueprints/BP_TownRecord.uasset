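; BP_TownRecord is an interactable record that opens a linear dialogue in interpretation mode, offering a two-way choice when it counts as evidence.
; Overlap ranges toggle a prompt and a discovery glow for the player, the glow only until MarkRecorded is called.
; Interact respects repeat and consumed flags, then registers the dialogue widget and itself on the player character unless one is active.
; Its mesh is invisible and non-colliding at runtime.
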(event OnComponentBeginOverlap(PromptRange)
  (params (OverlappedComponent :type Primitive%20Component%20Object%20Reference) (OtherActor :type Actor%20Object%20Reference) (OtherComp :type Primitive%20Component%20Object%20Reference) (OtherBodyIndex :type Integer) (bFromSweep :type Boolean) (SweepResult :type Hit%20Result%20Structure%20%28by%20ref%29))
  (if (== OtherActor (Game|Player|GetPlayerPawn 0))
    (Development|SetHiddeninGame (Variables|Default|GetPromptText) false false)))

(event OnComponentEndOverlap(PromptRange)
  (params (OverlappedComponent :type Primitive%20Component%20Object%20Reference) (OtherActor :type Actor%20Object%20Reference) (OtherComp :type Primitive%20Component%20Object%20Reference) (OtherBodyIndex :type Integer))
  (if (== OtherActor (Game|Player|GetPlayerPawn 0))
    (Development|SetHiddeninGame (Variables|Default|GetPromptText) true false)))

(event OnComponentBeginOverlap(DiscoveryRange)
  (params (OverlappedComponent :type Primitive%20Component%20Object%20Reference) (OtherActor :type Actor%20Object%20Reference) (OtherComp :type Primitive%20Component%20Object%20Reference) (OtherBodyIndex :type Integer) (bFromSweep :type Boolean) (SweepResult :type Hit%20Result%20Structure%20%28by%20ref%29))
  (if (and (== OtherActor (Game|Player|GetPlayerPawn 0)) (not (Variables|Default|GetbRecorded)))
    (Development|SetHiddeninGame (Variables|Default|GetDiscoveryGlow) false false)))

(event OnComponentEndOverlap(DiscoveryRange)
  (params (OverlappedComponent :type Primitive%20Component%20Object%20Reference) (OtherActor :type Actor%20Object%20Reference) (OtherComp :type Primitive%20Component%20Object%20Reference) (OtherBodyIndex :type Integer))
  (if (== OtherActor (Game|Player|GetPlayerPawn 0))
    (Development|SetHiddeninGame (Variables|Default|GetDiscoveryGlow) true false)))

(event Collision|EventActorBeginOverlap
  (params (OtherActor :type Actor%20Object%20Reference))
  (|CallParentFunction OtherActor))

(event EventTick
  (params (DeltaSeconds :type Float%20%28single-precision%29))
  (|CallParentFunction DeltaSeconds))

(event EventInteract
  (params (Instigator :type Actor%20Object%20Reference))
  (if (or (Variables|Conversation|GetbCanRepeat) (not (Variables|Conversation|GetbConsumed)))
    (CallFunction|OpenConversation)))

(event EventBeginPlay
  (Rendering|SetVisibility (Variables|Character|GetMesh) false true)
  (Collision|SetCollisionEnabled (Variables|Character|GetMesh) "NoCollision"))

(fn ConstructionScript
  (|CallParentFunction))

(fn OpenConversation
  (bind _asbp_third_person_character (Utilities|Casting|CastToBP_ThirdPersonCharacter (Game|Player|GetPlayerPawn 0)))
  (Utilities|IsValid (Variables|/Game/ThirdPerson/Blueprints/BP_ThirdPersonCharacter.BP_ThirdPersonCharacter_C|GetActiveDialogue _asbp_third_person_character)
    (:Is%20Not%20Valid
      (bind _returnvalue (UserInterface|CreateWidget "/Game/Week8/WBP_DialogueLinear.WBP_DialogueLinear_C" (Game|GetPlayerController 0) 0))
      (Variables|/Game/Week8/WBP_DialogueLinear.WBP_DialogueLinear_C|SetDialogueTable _returnvalue (Variables|Conversation|GetDialogueTable))
      (Variables|/Game/ThirdPerson/Blueprints/BP_ThirdPersonCharacter.BP_ThirdPersonCharacter_C|SetActiveDialogue _asbp_third_person_character _returnvalue)
      (Variables|/Game/ThirdPerson/Blueprints/BP_ThirdPersonCharacter.BP_ThirdPersonCharacter_C|SetActiveSpeaker _asbp_third_person_character self)
      (Variables|/Game/ThirdPerson/Blueprints/BP_ThirdPersonCharacter.BP_ThirdPersonCharacter_C|SetbCloseNext _asbp_third_person_character false)
      (Variables|/Game/Week8/WBP_DialogueLinear.WBP_DialogueLinear_C|SetbOfferChoice _returnvalue (Variables|Conversation|GetbCountsAsEvidence))
      (Variables|/Game/Week8/WBP_DialogueLinear.WBP_DialogueLinear_C|SetbInterpretationMode _returnvalue true)
      (Variables|/Game/Week8/WBP_DialogueLinear.WBP_DialogueLinear_C|SetbFinalChoice _returnvalue false)
      (Variables|/Game/Week8/WBP_DialogueLinear.WBP_DialogueLinear_C|SetChoiceA _returnvalue (Variables|Conversation|GetChoiceA))
      (Variables|/Game/Week8/WBP_DialogueLinear.WBP_DialogueLinear_C|SetChoiceB _returnvalue (Variables|Conversation|GetChoiceB))
      (Variables|/Game/Week8/WBP_DialogueLinear.WBP_DialogueLinear_C|SetChoicePrompt _returnvalue (Variables|Conversation|GetChoicePrompt))
      (Variables|/Game/Week8/WBP_DialogueLinear.WBP_DialogueLinear_C|SetOpinionA _returnvalue (Variables|Default|GetOpinionA))
      (Variables|/Game/Week8/WBP_DialogueLinear.WBP_DialogueLinear_C|SetOpinionB _returnvalue (Variables|Default|GetOpinionB))
      (Variables|/Game/Week8/WBP_DialogueLinear.WBP_DialogueLinear_C|SetResponseA _returnvalue (Variables|Default|GetResponseA))
      (Variables|/Game/Week8/WBP_DialogueLinear.WBP_DialogueLinear_C|SetResponseB _returnvalue (Variables|Default|GetResponseB))
      (UserInterface|Viewport|AddtoViewport _returnvalue 10)
      (Default|BeginDialogue _returnvalue))))

(fn MarkRecorded
  (Variables|Default|SetbRecorded true)
  (Development|SetHiddeninGame (Variables|Default|GetDiscoveryGlow) true false))