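; BP_PrototypeProgressManager is an actor that tracks prototype progress through collected evidence and a death notice read flag.
; RegisterEvidence adds unseen IDs to CollectedEvidenceIDs, updates EvidenceCount, and sets LastAdded to show whether the ID was new.
; MarkDeathNoticeRead sets ReadDeathNotice.
; An unreached copy of the registration logic also sets PrototypeComplete at an evidence threshold, but the live path never sets it.
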(event EventBeginPlay)

(event Collision|EventActorBeginOverlap
  (params (OtherActor :type Actor%20Object%20Reference)))

(event EventTick
  (params (DeltaSeconds :type Float%20%28single-precision%29)))

(fn ConstructionScript)

(fn RegisterEvidence
  (params (EvidenceID :type Name))
  (Variables|Progress|SetbLastAdded false)
  (if (not (Utilities|Array|ContainsItem (Variables|Progress|GetCollectedEvidenceIDs) EvidenceID))
    (Utilities|Array|Add (Variables|Progress|GetCollectedEvidenceIDs) EvidenceID)
    (Variables|Progress|SetbLastAdded true)
    (Variables|Progress|SetEvidenceCount (Utilities|Array|Length (Variables|Progress|GetCollectedEvidenceIDs)))))

(fn MarkDeathNoticeRead
  (Variables|Progress|SetbReadDeathNotice true))