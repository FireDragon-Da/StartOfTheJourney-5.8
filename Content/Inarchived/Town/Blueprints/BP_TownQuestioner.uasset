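; Town NPC that greets the player and runs the questioner conversation, including the game's final leave-or-remain choice.
; Proximity overlap turns it toward the player once and plays a wave montage, while TalkRange toggles a talk prompt.
; Talk reads BP_PrototypeProgressManager, picks the ending, redirect or after-choice dialogue table based on evidence and completion, then fills and opens a WBP_DialogueLinear widget registered on the player character.
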(event OnComponentBeginOverlap(Proximity)
  (params (OverlappedComponent :type Primitive%20Component%20Object%20Reference) (OtherActor :type Actor%20Object%20Reference) (OtherComp :type Primitive%20Component%20Object%20Reference) (OtherBodyIndex :type Integer) (bFromSweep :type Boolean) (SweepResult :type Hit%20Result%20Structure%20%28by%20ref%29))
  (if (and (== OtherActor (Game|Player|GetPlayerPawn 0)) (not (Variables|Default|GetHasGreeted)))
    (Variables|Default|SetHasGreeted true)
    (Transformation|SetActorRotation self (Math|Rotator|MakeRotator 0.0 0.0 (.Yaw (Math|Rotator|BreakRotator (Math|Rotator|FindLookatRotation (Transformation|GetActorLocation) (Transformation|GetActorLocation OtherActor))))))
    (Utilities|FlowControl|Delay 0.4)
    (Animation|Montage|MontagePlay (Components|SkeletalMesh|GetAnimInstance (Variables|Default|GetMesh)) (Variables|Default|GetWaveMontage) 1.0 "MontageLength" 0.0 false)))

(event OnComponentBeginOverlap(TalkRange)
  (params (OverlappedComponent :type Primitive%20Component%20Object%20Reference) (OtherActor :type Actor%20Object%20Reference) (OtherComp :type Primitive%20Component%20Object%20Reference) (OtherBodyIndex :type Integer) (bFromSweep :type Boolean) (SweepResult :type Hit%20Result%20Structure%20%28by%20ref%29))
  (if (== OtherActor (Game|Player|GetPlayerPawn 0))
    (Development|SetHiddeninGame (Variables|Default|GetPromptText) false false)))

(event OnComponentEndOverlap(TalkRange)
  (params (OverlappedComponent :type Primitive%20Component%20Object%20Reference) (OtherActor :type Actor%20Object%20Reference) (OtherComp :type Primitive%20Component%20Object%20Reference) (OtherBodyIndex :type Integer))
  (if (== OtherActor (Game|Player|GetPlayerPawn 0))
    (Development|SetHiddeninGame (Variables|Default|GetPromptText) true false)))

(event EventBeginPlay)

(event Collision|EventActorBeginOverlap
  (params (OtherActor :type Actor%20Object%20Reference)))

(event EventTick
  (params (DeltaSeconds :type Float%20%28single-precision%29)))

(fn ConstructionScript)

(fn Talk
  (bind _asbp_third_person_character (Utilities|Casting|CastToBP_ThirdPersonCharacter (Game|Player|GetPlayerPawn 0)))
  (Utilities|IsValid (Variables|/Game/ThirdPerson/Blueprints/BP_ThirdPersonCharacter.BP_ThirdPersonCharacter_C|GetActiveDialogue _asbp_third_person_character)
    (:Is%20Not%20Valid
      (bind _outactors (Actor|GetAllActorsOfClass "/Game/Inarchived/Blueprints/BP_PrototypeProgressManager.BP_PrototypeProgressManager_C"))
      (bind _asbp_prototype_progress_manager (Utilities|Casting|CastToBP_PrototypeProgressManager (Utilities|Array|Get(acopy) _outactors)))
      (bind _returnvalue (UserInterface|CreateWidget "/Game/Week8/WBP_DialogueLinear.WBP_DialogueLinear_C" (Game|GetPlayerController 0) 0))
      (if (and (Variables|/Game/Inarchived/Blueprints/BP_PrototypeProgressManager.BP_PrototypeProgressManager_C|GetbReadDeathNotice _asbp_prototype_progress_manager) (and (Utilities|Array|ContainsItem (Variables|/Game/Inarchived/Blueprints/BP_PrototypeProgressManager.BP_PrototypeProgressManager_C|GetCollectedEvidenceIDs _asbp_prototype_progress_manager) "PhotoAfterDeath") (Utilities|Array|ContainsItem (Variables|/Game/Inarchived/Blueprints/BP_PrototypeProgressManager.BP_PrototypeProgressManager_C|GetCollectedEvidenceIDs _asbp_prototype_progress_manager) "WitnessRecording")))
        (Variables|/Game/Week8/WBP_DialogueLinear.WBP_DialogueLinear_C|SetDialogueTable _returnvalue "/Game/Inarchived/Dialogue/DT_GuyEnding.DT_GuyEnding")
        (else
          (Variables|/Game/Week8/WBP_DialogueLinear.WBP_DialogueLinear_C|SetDialogueTable _returnvalue "/Game/Inarchived/Dialogue/DT_GuyRedirect.DT_GuyRedirect")))
      (Variables|/Game/ThirdPerson/Blueprints/BP_ThirdPersonCharacter.BP_ThirdPersonCharacter_C|SetActiveDialogue _asbp_third_person_character _returnvalue)
      (Variables|/Game/ThirdPerson/Blueprints/BP_ThirdPersonCharacter.BP_ThirdPersonCharacter_C|SetActiveSpeaker _asbp_third_person_character self)
      (Variables|/Game/ThirdPerson/Blueprints/BP_ThirdPersonCharacter.BP_ThirdPersonCharacter_C|SetbCloseNext _asbp_third_person_character false)
      (Variables|/Game/Week8/WBP_DialogueLinear.WBP_DialogueLinear_C|SetbInterpretationMode _returnvalue true)
      (Variables|/Game/Week8/WBP_DialogueLinear.WBP_DialogueLinear_C|SetbFinalChoice _returnvalue (and (Variables|/Game/Inarchived/Blueprints/BP_PrototypeProgressManager.BP_PrototypeProgressManager_C|GetbReadDeathNotice _asbp_prototype_progress_manager) (and (Utilities|Array|ContainsItem (Variables|/Game/Inarchived/Blueprints/BP_PrototypeProgressManager.BP_PrototypeProgressManager_C|GetCollectedEvidenceIDs _asbp_prototype_progress_manager) "PhotoAfterDeath") (Utilities|Array|ContainsItem (Variables|/Game/Inarchived/Blueprints/BP_PrototypeProgressManager.BP_PrototypeProgressManager_C|GetCollectedEvidenceIDs _asbp_prototype_progress_manager) "WitnessRecording"))))
      (Variables|/Game/Week8/WBP_DialogueLinear.WBP_DialogueLinear_C|SetbOfferChoice _returnvalue true)
      (if (and (Variables|/Game/Inarchived/Blueprints/BP_PrototypeProgressManager.BP_PrototypeProgressManager_C|GetbReadDeathNotice _asbp_prototype_progress_manager) (and (Utilities|Array|ContainsItem (Variables|/Game/Inarchived/Blueprints/BP_PrototypeProgressManager.BP_PrototypeProgressManager_C|GetCollectedEvidenceIDs _asbp_prototype_progress_manager) "PhotoAfterDeath") (Utilities|Array|ContainsItem (Variables|/Game/Inarchived/Blueprints/BP_PrototypeProgressManager.BP_PrototypeProgressManager_C|GetCollectedEvidenceIDs _asbp_prototype_progress_manager) "WitnessRecording")))
        (Variables|/Game/Week8/WBP_DialogueLinear.WBP_DialogueLinear_C|SetChoicePrompt _returnvalue "The photograph and the voice cannot settle it for you. What will you choose?")
        (Variables|/Game/Week8/WBP_DialogueLinear.WBP_DialogueLinear_C|SetChoiceA _returnvalue "Leave. My choice does not need a certificate from this town.")
        (Variables|/Game/Week8/WBP_DialogueLinear.WBP_DialogueLinear_C|SetChoiceB _returnvalue "Remain. An uncertain world still contains things I care about.")
        (Variables|/Game/Week8/WBP_DialogueLinear.WBP_DialogueLinear_C|SetOpinionA _returnvalue "Leave without certainty")
        (Variables|/Game/Week8/WBP_DialogueLinear.WBP_DialogueLinear_C|SetOpinionB _returnvalue "Remain by choice")
        (Variables|/Game/Week8/WBP_DialogueLinear.WBP_DialogueLinear_C|SetResponseA _returnvalue "You choose departure without calling the outside more real. The record can describe that choice; it cannot make it for you. END / LEAVE.")
        (Variables|/Game/Week8/WBP_DialogueLinear.WBP_DialogueLinear_C|SetResponseB _returnvalue "You remain without declaring the town true. Staying is your answer, not a verdict the archive gave you. END / REMAIN.")
        (else
          (Variables|/Game/Week8/WBP_DialogueLinear.WBP_DialogueLinear_C|SetChoicePrompt _returnvalue "What do you ask the man who was already expecting you?")
          (Variables|/Game/Week8/WBP_DialogueLinear.WBP_DialogueLinear_C|SetChoiceA _returnvalue "What kind of proof would you accept?")
          (Variables|/Game/Week8/WBP_DialogueLinear.WBP_DialogueLinear_C|SetChoiceB _returnvalue "Where did the town get its story about me?")
          (Variables|/Game/Week8/WBP_DialogueLinear.WBP_DialogueLinear_C|SetOpinionA _returnvalue "Question the judge")
          (Variables|/Game/Week8/WBP_DialogueLinear.WBP_DialogueLinear_C|SetOpinionB _returnvalue "Question the source")
          (Variables|/Game/Week8/WBP_DialogueLinear.WBP_DialogueLinear_C|SetResponseA _returnvalue "If I choose the standard, you will only prove you satisfy me. Read the notice, then bring the rooftop photograph and the radio above the north street. Tell me what YOU accept.")
          (Variables|/Game/Week8/WBP_DialogueLinear.WBP_DialogueLinear_C|SetResponseB _returnvalue "The notice, photograph, and radio borrowed authority from one another. Follow the floating routes above the north streets. Keep their contradictions instead of replacing one story with another.")))
      (if (Variables|/Game/Inarchived/Blueprints/BP_PrototypeProgressManager.BP_PrototypeProgressManager_C|GetbPrototypeComplete _asbp_prototype_progress_manager)
        (Variables|/Game/Week8/WBP_DialogueLinear.WBP_DialogueLinear_C|SetbOfferChoice _returnvalue false)
        (Variables|/Game/Week8/WBP_DialogueLinear.WBP_DialogueLinear_C|SetbFinalChoice _returnvalue false)
        (Variables|/Game/Week8/WBP_DialogueLinear.WBP_DialogueLinear_C|SetDialogueTable _returnvalue "/Game/Inarchived/Dialogue/DT_GuyAfterChoice.DT_GuyAfterChoice"))
      (UserInterface|Viewport|AddtoViewport _returnvalue 10)
      (Default|BeginDialogue _returnvalue))))