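; BP_TownSignpost is a town signpost actor that changes appearance with the current phase.
; ApplyPhase passes the phase to HandlePhase, which acts only when it is 1 or higher.
; It then turns the lantern light red and hides the second plate along with its text and tip components.
; There is no branch to restore the original look, and BeginPlay, overlap and Tick are unused.
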(event EventBeginPlay)

(event Collision|EventActorBeginOverlap
  (params (OtherActor :type Actor%20Object%20Reference)))

(event EventTick
  (params (DeltaSeconds :type Float%20%28single-precision%29)))

(event EventApplyPhase
  (params (CurrentPhase :type Integer))
  (CallFunction|HandlePhase CurrentPhase))

(fn ConstructionScript)

(fn HandlePhase
  (params (Phase :type Integer))
  (if (>= Phase 1)
    (Rendering|Components|Light|SetLightColor (Variables|Default|GetLanternLight) "(R=1.000000,G=0.150000,B=0.100000,A=1.000000)" true)
    (Rendering|SetVisibility (Variables|Default|GetPlateB) false false)
    (Rendering|SetVisibility (Variables|Default|GetPlateBText) false false)
    (Rendering|SetVisibility (Variables|Default|GetPlateBTip) false false)))