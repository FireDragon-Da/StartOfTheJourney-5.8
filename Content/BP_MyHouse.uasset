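; BP_MyHouse is a practice Blueprint that prints two variables to the screen on BeginPlay, before and after reassigning them.
; A disconnected node chain would build a simple house from runtime-added static mesh components: scaled cubes for foundation and four walls, two ramps for the roof.
; That chain has no triggering event, so it never runs, and the Construction Script is empty.
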(event EventBeginPlay
  (Development|PrintString (Utilities|String|ToString(Integer) (Variables|Default|GetmyFirstVar)) true true "(R=0.000000,G=0.660000,B=1.000000,A=1.000000)" 1e+01)
  (bind _output_get (Variables|Default|SetmyFirstVar 2))
  (Development|PrintString (Utilities|String|Append "Second Var: " (Utilities|String|ToString(Integer) _output_get)) true true "(R=0.000000,G=0.660000,B=1.000000,A=1.000000)" 1e+01)
  (Development|PrintString (Utilities|String|ToString(Float) (Variables|Default|GetmySecondVar)) true true "(R=0.000000,G=0.660000,B=1.000000,A=1.000000)" 1e+01)
  (Variables|Default|SetmySecondVar 4.0)
  (Development|PrintString (Utilities|String|ToString(Float) (Variables|Default|GetmySecondVar)) true true "(R=0.000000,G=0.660000,B=1.000000,A=1.000000)" 1e+01))

(fn ConstructionScript)