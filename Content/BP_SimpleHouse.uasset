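; BP_SimpleHouse is an actor that assembles a simple house at runtime when another actor overlaps it.
; The overlap event adds seven static mesh components, using scaled cubes for the floor and four walls and two ramps for the roof.
; Nothing guards against repeat overlaps, so each one adds another set of meshes.
; BeginPlay separately sets and prints two test variables, and the construction script is empty.
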(event EventBeginPlay
  (Development|PrintString (Utilities|String|ToString(Integer) (Variables|Default|GetmyFirstVar)))
  (Variables|Default|SetmyFirstVar 2)
  (Development|PrintString (Utilities|String|Append "Second Var: " (Utilities|String|ToString(Integer) (Variables|Default|GetmyFirstVar))))
  (Development|PrintString (Utilities|String|ToString(Float) (Variables|Default|GetmySecondVar)))
  (Variables|Default|SetmySecondVar 4.0)
  (Development|PrintString (Utilities|String|ToString(Float) (Variables|Default|GetmySecondVar))))

(event Collision|EventActorBeginOverlap
  (params (OtherActor :type Actor%20Object%20Reference))
  (Development|PrintString "starting construction")
  (bind _returnvalue (AddComponent|AddStaticMeshComponent false))
  (Components|StaticMesh|SetStaticMesh _returnvalue "/Game/LevelPrototyping/Meshes/SM_Cube.SM_Cube")
  (Transformation|SetRelativeLocation _returnvalue "-20.000000,-30.000000,0.000000" false false)
  (Transformation|SetRelativeScale3D _returnvalue "1.500000,1.500000,0.100000")
  (bind _returnvalue_2 (AddComponent|AddStaticMeshComponent false))
  (Components|StaticMesh|SetStaticMesh _returnvalue_2 "/Game/LevelPrototyping/Meshes/SM_Cube.SM_Cube")
  (Transformation|SetRelativeScale3D _returnvalue_2 "0.100000,1.000000,1.000000")
  (bind _returnvalue_3 (AddComponent|AddStaticMeshComponent false))
  (Components|StaticMesh|SetStaticMesh _returnvalue_3 "/Game/LevelPrototyping/Meshes/SM_Cube.SM_Cube")
  (Transformation|SetRelativeLocation _returnvalue_3 "90.000000,0.000000,0.000000" false false)
  (Transformation|SetRelativeScale3D _returnvalue_3 "0.100000,1.000000,1.000000")
  (bind _returnvalue_4 (AddComponent|AddStaticMeshComponent false))
  (Components|StaticMesh|SetStaticMesh _returnvalue_4 "/Game/LevelPrototyping/Meshes/SM_Cube.SM_Cube")
  (Transformation|SetRelativeScale3D _returnvalue_4 "1.000000,0.100000,1.000000")
  (bind _returnvalue_5 (AddComponent|AddStaticMeshComponent false))
  (Components|StaticMesh|SetStaticMesh _returnvalue_5 "/Game/LevelPrototyping/Meshes/SM_Cube.SM_Cube")
  (Transformation|SetRelativeLocation _returnvalue_5 "0.000000,90.000000,0.000000" false false)
  (Transformation|SetRelativeScale3D _returnvalue_5 "1.000000,0.100000,1.000000")
  (bind _returnvalue_6 (AddComponent|AddStaticMeshComponent false))
  (Components|StaticMesh|SetStaticMesh _returnvalue_6 "/Game/LevelPrototyping/Meshes/SM_Ramp.SM_Ramp")
  (Transformation|SetRelativeLocation _returnvalue_6 "0.000000,50.000000,100.000000" false false)
  (Transformation|SetRelativeScale3D _returnvalue_6 "1.000000,0.500000,0.500000")
  (bind _returnvalue_7 (AddComponent|AddStaticMeshComponent false))
  (Components|StaticMesh|SetStaticMesh _returnvalue_7 "/Game/LevelPrototyping/Meshes/SM_Ramp.SM_Ramp")
  (Transformation|SetRelativeLocation _returnvalue_7 "100.000000,50.000000,100.000000" false false)
  (Transformation|SetRelativeRotation _returnvalue_7 "0.000000,180.000000,0.000000" false false)
  (Transformation|SetRelativeScale3D _returnvalue_7 "1.000000,0.500000,0.500000"))

(fn ConstructionScript)